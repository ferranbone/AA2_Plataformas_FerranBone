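; Jetpack logic that runs on its owning BP_ThirdPersonCharacter and gives it fuel-limited upward thrust.
; Each Tick applies a small additive LaunchCharacter boost while the character is falling with HasJetpack and Saltando set, draining JetpackEnergy.
; Energy recharges when not falling, without a cap because the clamp node is unconnected.
; The energy ratio drives the EnergyAmount parameter on the character's MaterialJetpack.
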(event EventBeginPlay)

(event EventTick
  (params (DeltaSeconds :type Float%20%28single-precision%29))
  (bind _asbp_third_person_character (Utilities|Casting|CastToBP_ThirdPersonCharacter (Components|GetOwner)))
  (Rendering|Material|SetScalarParameterValue (Variables|/Game/CORREGIR/BP_ThirdPersonCharacter.BP_ThirdPersonCharacter_C|GetMaterialJetpack _asbp_third_person_character) "EnergyAmount" (/ (Variables|Default|GetJetpackEnergy) (Variables|Default|GetMaxJetpackEnergy)) :!class /Script/Engine.MaterialInstanceDynamic)
  (if (AI|Components|NavMovement|IsFalling (Variables|/Script/Engine.Character|GetCharacterMovement _asbp_third_person_character))
    (if (Math|Boolean|ANDBoolean (Variables|/Game/CORREGIR/BP_ThirdPersonCharacter.BP_ThirdPersonCharacter_C|GetHasJetpack _asbp_third_person_character) (> (Variables|Default|GetJetpackEnergy) 0.0) (Variables|/Game/CORREGIR/BP_ThirdPersonCharacter.BP_ThirdPersonCharacter_C|GetSaltando _asbp_third_person_character))
      (Character|LaunchCharacter _asbp_third_person_character "0.000000,0.000000,15.000000" false false)
      (Variables|Default|SetJetpackEnergy (- (Variables|Default|GetJetpackEnergy) (* DeltaSeconds (Variables|Default|GetEnergyUseRate)))))
    (else
      (Variables|Default|SetJetpackEnergy (+ (Variables|Default|GetJetpackEnergy) (* DeltaSeconds (Variables|Default|GetRechargeRate)))))))