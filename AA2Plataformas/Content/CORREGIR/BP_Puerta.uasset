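; BP_Puerta is a goal door that reports a win and plays a sound when the third-person character overlaps its box with at least two keys.
; A custom event counts collected keys, starting audio and a timer widget on the first and stopping the audio on later ones.
; Each call also sets a timer that reopens ThirdPersonMap if fewer than two keys are held when it fires.
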(event OnComponentBeginOverlap(Box)
  (params (OverlappedComponent :type Primitive%20Component%20Object%20Reference) (OtherActor :type Actor%20Object%20Reference) (OtherComp :type Primitive%20Component%20Object%20Reference) (OtherBodyIndex :type Integer) (bFromSweep :type Boolean) (SweepResult :type Hit%20Result%20Structure%20%28by%20ref%29))
  (Utilities|Casting|CastToBP_ThirdPersonCharacter OtherActor)
  (if (>= (Variables|Default|GetKeysCollected) 2)
    (Development|PrintString "Has ganado!")
    (Audio|PlaySoundatLocation "/Game/CORREGIR/Audio/metaPuerta.metaPuerta" "0, 0, 0" "0, 0, 0" 1.0 1.0 0.0 0 0 0 0)
    (else
      (Development|PrintString "Puerta cerrada"))))

(event Custom|CustomEvent
  (bind _output_get (Variables|Default|SetKeysCollected (+ (Variables|Default|GetKeysCollected) 1)))
  (if (== _output_get 1)
    (Audio|Components|Audio|Play (Variables|Default|GetAudio) 0.0)
    (bind _returnvalue (UserInterface|CreateWidget "/Game/CORREGIR/Timer.Timer_C"))
    (UserInterface|Viewport|AddtoViewport _returnvalue 0)
    (else
      (Audio|Components|Audio|Stop (Variables|Default|GetAudio))))
  (Utilities|Time|SetTimerbyEvent (delegate Custom|Restart) (Variables|Default|GetTiempoKeys)))

(event Custom|Restart
  (if (not (>= (Variables|Default|GetKeysCollected) 2))
    (Game|OpenLevel(byName) "ThirdPersonMap")))

(event EventBeginPlay)

(event Collision|EventActorBeginOverlap
  (params (OtherActor :type Actor%20Object%20Reference)))

(fn ConstructionScript)